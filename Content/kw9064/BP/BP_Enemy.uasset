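; BP_Enemy is an enemy pawn that chases the player and can be killed by damage.
; On BeginPlay it uses AI MoveTo toward the player character and destroys itself two seconds after reaching them.
; AnyDamage subtracts from EnemyHP, prints the remaining value, and destroys the actor at zero or below.
; An emitter spawn node is left unconnected, so no effect plays.
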(event `self.ReceiveBeginPlay`
  ;[1 1 1] 시작하자마자 플레이어를 따라와라
  (`self.Ev_ChasePlayer`))

(event `Ev_ChasePlayer`
  ;[1 1 1] 플레이어와 접촉하면 2초후 파괴
  (`|AIMoveTo` self (0.0 0.0 0.0) (`GameplayStatics.GetPlayerCharacter` 0) 1.0
    (:`OnSuccess`
      (`KismetSystemLibrary.Delay` 2.0)
      (`self.K2_DestroyActor`))))

(event `self.ReceiveAnyDamage`
  (params (Damage :type "Float (single-precision)") (DamageType :type "DamageType Object Reference") (InstigatedBy :type "Controller Object Reference") (DamageCauser :type "Actor Object Reference"))
  ;[1 1 1] 적을 공격했을 때 파괴
  (bind _output_get (set `self.EnemyHP` (- (`self.EnemyHP`) Damage)))
  (`KismetSystemLibrary.PrintString` (`KismetStringLibrary.Conv_DoubleToString` _output_get))
  (if (<= (`self.EnemyHP`) 0.0)
    (`self.K2_DestroyActor`)))

(fn `UserConstructionScript`)